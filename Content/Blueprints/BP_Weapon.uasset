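; BP_Weapon is a weapon that fires projectiles and grenades and carries a toggleable spotlight.
; Both spawn events take location and direction from CalcFireInfo to place BP_Projectile or BP_Grenade.
; Projectiles spawn only when CalcFireInfo returns true, while grenades always spawn.
; ChangeSpots flips IsSpot, which Tick reads every frame to switch the spotlight intensity between full and zero.
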(event `self.Spawn_grenade`
  (bind (_location _dir) (`self.Calc_Fire_Info`))
  (if true
    (`|SpawnActorFromClass` "/Game/Blueprints/BP_Grenade.BP_Grenade_C" (`KismetMathLibrary.MakeTransform` _location (`KismetMathLibrary.Conv_VectorToRotator` _dir)) "Undefined" "OverrideRootScale" null null)))

(event `self.Spawn_Projectile`
  (bind (_location _dir _returnvalue) (`self.Calc_Fire_Info`))
  (if _returnvalue
    (`|SpawnActorFromClass` "/Game/Blueprints/BP_Projectile.BP_Projectile_C" (`KismetMathLibrary.MakeTransform` _location (`KismetMathLibrary.Conv_VectorToRotator` _dir) (1.0 1.0 1.0)) "Undefined" "OverrideRootScale" null null)))

(event `self.ReceiveTick`
  (params (DeltaSeconds :type "Float (single-precision)"))
  (if (`self.Is_spot`)
    (`LightComponent.SetIntensity` (`self.SpotLight`) 25000.0)
    (else
      (`LightComponent.SetIntensity` (`self.SpotLight`) 0.0))))

(event `self.change_spots`
  (set `self.Is_spot` (not (`self.Is_spot`))))

(fn `UserConstructionScript`)