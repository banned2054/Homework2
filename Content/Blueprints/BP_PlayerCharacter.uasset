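; Player character Blueprint that spawns and attaches a weapon, creates the on-screen widget and ends the game when the player leaves the play area.
; Fire start, spot change and grenade events forward to the weapon, while stopping fire only clears the firing flag.
; Tick checks hard-coded X/Y bounds; outside them it calls the widget's END, then TrueEnd after a delay, and quits after another.
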(event `self.ReceiveBeginPlay`
  (bind _returnvalue (`|SpawnActorFromClass` (`self.weapon_class`) (`KismetMathLibrary.MakeTransform` (0.0 0.0 0.0)) "Undefined" "OverrideRootScale" null null))
  (bind _output_get (set `self.Weapon` _returnvalue))
  (`self.K2_AttachToComponent` _output_get (`self.attach_Weapon`) "None" "KeepRelative" "KeepRelative" "KeepRelative" true)
  (bind _returnvalue_2 (`|CreateWidget` "/Game/Blueprints/BP_Widget.BP_Widget_C"))
  (bind _output_get_2 (set `self.Widget` _returnvalue_2))
  (`UserWidget.AddToViewport` _output_get_2 0))

(event `self.Start_fire`
  (set `self.is_fire` true)
  (`Weapon.Start_fire` (`self.Weapon`)))

(event `self.Stop_fire`
  (set `self.is_fire` false))

(event `self.ReceiveTick`
  (params (DeltaSeconds :type "Float (single-precision)"))
  (bind _widget (`self.Widget`))
  (bind _x (.x (.location (`self.GetTransform`))))
  (bind _y (.y (.location (`self.GetTransform`))))
  (if (or (< _x -1940.0) (> _x 1140.0) (< _y -1530.0) (> _y 1530.0))
    (`/Game/Blueprints/BP_Widget.END_` _widget)
    (`KismetSystemLibrary.Delay` 15.0)
    (`/Game/Blueprints/BP_Widget.True_end` _widget)
    (`KismetSystemLibrary.Delay` 10.0)
    (`KismetSystemLibrary.QuitGame` null "Quit")))

(event `self.Change_spot`
  (`Weapon.Change_spot` (`self.Weapon`)))

(event `self.Start_grenade`
  (`Weapon.Start_grenade` (`self.Weapon`)))

(fn `UserConstructionScript`)